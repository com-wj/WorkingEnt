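; Test pushable block actor that slides along world X or Y when hit, based on which horizontal axis the hit normal matches.
; Four timelines, one per direction, offset the block from its stored start location without sweeping.
; A BlockMoving flag blocks further pushes until a one-second Delay, triggered from timeline updates, re-caches the location and clears it.
; Hits matching no axis leave the flag set.
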(event EventBeginPlay
  (Variables|Default|SetInit%20Box%20Location (Transformation|GetActorLocation))
  (Variables|Default|Setblock_moving false))

(event Collision|EventHit
  (params (MyComp :type Primitive%20Component%20Object%20Reference) (Other :type Actor%20Object%20Reference) (OtherComp :type Primitive%20Component%20Object%20Reference) (bSelfMoved :type Boolean) (HitLocation :type Vector :default "0, 0, 0") (HitNormal :type Vector :default "0, 0, 0") (NormalImpulse :type Vector :default "0, 0, 0") (Hit :type Hit%20Result%20Structure%20%28by%20ref%29))
  (if (not (Variables|Default|Getblock_moving))
    (Variables|Default|Setblock_moving true)
    (if (Math|Vector|Equal(Vector) HitNormal "1.000000, 0, 0" 0.5)
      (bind _새_트랙_0 (Timeline|타임라인_0 PlayFromStart)
        (:Update
          (Transformation|SetActorLocation (+ _새_트랙_0 (Variables|Default|GetInit%20Box%20Location)) false false)
          (Utilities|FlowControl|Delay 1.0 :!label _label)
          (Variables|Default|SetInit%20Box%20Location (Transformation|GetActorLocation))
          (Variables|Default|Setblock_moving false)))
      (elif (Math|Vector|Equal(Vector) HitNormal "-1.000000,0.000000, 0" 0.5)
        (bind _새_트랙_0_2 (Timeline|타임라인_1 PlayFromStart)
          (:Update
            (Transformation|SetActorLocation (+ _새_트랙_0_2 (Variables|Default|GetInit%20Box%20Location)) false false)
            (goto _label)))
        (elif (Math|Vector|Equal(Vector) HitNormal "0,1.000000, 0" 0.5)
          (bind _새_트랙_0_3 (Timeline|타임라인_2 PlayFromStart)
            (:Update
              (Transformation|SetActorLocation (+ _새_트랙_0_3 (Variables|Default|GetInit%20Box%20Location)) false false)
              (goto _label)))
          (elif (Math|Vector|Equal(Vector) HitNormal "0,-1.000000,0.000000" 0.5)
            (bind _새_트랙_0_4 (Timeline|타임라인_3 PlayFromStart)
              (:Update
                (Transformation|SetActorLocation (+ _새_트랙_0_4 (Variables|Default|GetInit%20Box%20Location)) false false)
                (goto _label)))))))))

(fn ConstructionScript)